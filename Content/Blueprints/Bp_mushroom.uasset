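; Mushroom actor that grows in random steps after it spawns, using a mesh component named SMGenericTree02.
; BeginPlay runs a delayed loop that waits a random few seconds, adds a small random amount to the mesh's relative scale, and decrements GrowCounter until it reaches zero.
; A disconnected chain of random rescales is never run, and the construction script is empty.
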(event `self.ReceiveBeginPlay`
  (if (> (`self.GrowCounter`) 0) :!label _label
    (`KismetSystemLibrary.Delay` (`KismetMathLibrary.RandomFloatInRange` 1.0 3.0))
    (`SceneComponent.SetRelativeScale3D` (`self.SM_Generic_Tree_02`) (+ (`SceneComponent.RelativeScale3D` (`self.SM_Generic_Tree_02`)) (`KismetMathLibrary.RandomFloatInRange` 0.1 0.2)))
    (`SceneComponent.SetRelativeScale3D` (`self.SM_Generic_Tree_02`) (+ (`SceneComponent.RelativeScale3D` (`self.SM_Generic_Tree_02`)) (`KismetMathLibrary.RandomFloatInRange` 0.1 0.2)))
    (`/Engine/EditorBlueprintResources/StandardMacros.DecrementInt` (`self.GrowCounter`)
      (:`  `
        (goto _label)))))

(fn `UserConstructionScript`)