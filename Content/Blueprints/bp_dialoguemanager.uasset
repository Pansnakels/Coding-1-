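; Dialogue manager Blueprint that shows lines from a Dialogue array one at a time.
; Each DisplayNextLine call prints the entry at Index as purple debug text via PrintText, then increments Index until the array is exhausted.
; Once past the last line, further calls do nothing, as the node that resets Index to zero is unconnected and never runs.
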(event `DisplayNextLine`
  (if (not (>= (`self.Index`) (`KismetArrayLibrary.Array_Length` (`self.Dialogue`))))
    (`KismetSystemLibrary.PrintText` (`|GetArrayItem` (`self.Dialogue`) (`self.Index`)) true true (struct :`R` 0.436773 :`G` 0.022913 :`B` 1.0 :`A` 1.0) 5.0)
    (`/Engine/EditorBlueprintResources/StandardMacros.IncrementInt` (`self.Index`)) ; increment int
  ))

(fn `UserConstructionScript`)