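; Demo Blueprint for loops and arrays that runs two delayed routines on BeginPlay.
; After two seconds, a while loop counts WhileCounter down to zero, printing each value in a color picked from the Colors array by modulo.
; After one second, MakeCoinsJump raises every Bp_key actor, prints the count, then re-calls itself after a delay, so the keys keep climbing indefinitely.
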(event `self.ReceiveBeginPlay`
  (bind _whilecounter (`self.whileCounter`))
  (`|ExecutionSequence`
    (:`then_0`
      (`KismetSystemLibrary.Delay` 2.0)
      (while (> _whilecounter 0)
        (`KismetSystemLibrary.PrintText` (`|FormatText` "We are in loop number {count}." _whilecounter) true true (`|GetArrayItem` (`self.Colors`) (mod (`self.whileCounter`) 7)) 22.0)
        (`/Engine/EditorBlueprintResources/StandardMacros.DecrementInt` (`self.whileCounter`))))
    (:`then_1`
      (`KismetSystemLibrary.Delay` 1.0)
      (`self.MakeCoinsJump`))))

(event `MakeCoinsJump`
  (bind _outactors (`GameplayStatics.GetAllActorsOfClass` "/Game/Blueprints/bp_key.bp_key_C"))
  (for _array_element _outactors
    (`SceneComponent.K2_AddRelativeLocation` (`/Game/Blueprints/bp_key.DefaultSceneRoot` _array_element) (0.0 0.0 50.0) false false))
  (`KismetSystemLibrary.PrintText` (`|FormatText` "We have raise {count} Keys." (`KismetArrayLibrary.Array_Length` _outactors)) true true (struct :`G` 0.66 :`B` 1.0 :`A` 1.0) 30.0)
  (`KismetSystemLibrary.Delay` 1.0)
  (`self.MakeCoinsJump`))

(fn `UserConstructionScript`)