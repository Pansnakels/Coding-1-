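; Skeleton quest-giver that tracks the player's planting progress and hands out cabin keys, giving feedback through on-screen printed text.
; Its Playerhit event checks the player's planted tree count, then mushroom count, to choose between a tree prompt, a mushroom prompt or a forgiveness message.
; The latter two stages each use a DoOnce to spawn a Bp_key in front of the skeleton and set the player's TalktoSkeleton flag.
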(event `/Game/Blueprints/bp_i_interactions.Playerhit`
  (params (Player :type "/Game/ThirdPerson/Blueprints/BP_ThirdPersonCharacter Object Reference"))
  (set `self.Player` Player)
  (if (< (`/Game/ThirdPerson/Blueprints/BP_ThirdPersonCharacter.treesplanted` Player) 10)
    (`KismetSystemLibrary.PrintString` "Plant more trees!" true true (struct :`R` 0.046189 :`G` 1.0 :`A` 1.0) 3.0)
    (elif (< (`/Game/ThirdPerson/Blueprints/BP_ThirdPersonCharacter.Mushroomsplanted` Player) 5)
      (`KismetSystemLibrary.PrintString` "Now you need to plant 5 mushrooms!" true true (struct :`G` 1.0 :`B` 0.255257 :`A` 1.0))
      (`/Engine/EditorBlueprintResources/StandardMacros.DoOnce` false
        (:`Completed`
          (`KismetSystemLibrary.PrintString` "Here's the key to the cabin." true true (struct :`R` 0.241065 :`G` 1.0 :`B` 0.504782 :`A` 1.0) 5.0)
          (`|SpawnActorFromClass` "/Game/Blueprints/bp_key.bp_key_C" (`KismetMathLibrary.MakeTransform` (+ (`self.K2_GetActorLocation`) (* (`self.GetActorForwardVector`) 250.0))) "Undefined" "MultiplyWithRoot" null null)
          (set `/Game/ThirdPerson/Blueprints/BP_ThirdPersonCharacter.TalktoSkeleton` true (`self.Player`))))
      (else
        (`KismetSystemLibrary.PrintString` "Goodjob! I forgive you and now we can party!! " true true (struct :`R` 0.004252 :`G` 1.0 :`A` 1.0) 5.0)
        (`/Engine/EditorBlueprintResources/StandardMacros.DoOnce` false
          (:`Completed`
            (`KismetSystemLibrary.Delay` 2.0)
            (`KismetSystemLibrary.PrintString` "This is to the backdoor in the cabin, go party in the real world." true true (struct :`R` 0.687899 :`B` 1.0 :`A` 1.0) 15.0)
            (`|SpawnActorFromClass` "/Game/Blueprints/bp_key.bp_key_C" (`KismetMathLibrary.MakeTransform` (+ (`self.K2_GetActorLocation`) (* (`self.GetActorForwardVector`) 250.0))) "Undefined" "MultiplyWithRoot" null null)
            (set `/Game/ThirdPerson/Blueprints/BP_ThirdPersonCharacter.TalktoSkeleton` true (`self.Player`))))))))

(fn `UserConstructionScript`)