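; Door actor that a third-person character unlocks with a key and that then swings open and closed.
; On overlap, it spends one of the character's TotalKeys and sets IsUnlocked, printing feedback either way, with no check for an already unlocked door.
; A custom event, NewFunction, uses a FlipFlop to play or reverse a timeline once unlocked, lerping the mesh's yaw through a quarter turn.
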(event `self.ReceiveActorBeginOverlap`
  (params (OtherActor :type "Actor Object Reference"))
  (bind _asbp_third_person_character (cast `/Game/ThirdPerson/Blueprints/BP_ThirdPersonCharacter` OtherActor))
  (if (> (`/Game/ThirdPerson/Blueprints/BP_ThirdPersonCharacter.TotalKeys` _asbp_third_person_character) 0)
    (`/Engine/EditorBlueprintResources/StandardMacros.DecrementInt` (`/Game/ThirdPerson/Blueprints/BP_ThirdPersonCharacter.TotalKeys` _asbp_third_person_character) ; subtract 1 from total keys
      (:`  `
        (`KismetSystemLibrary.PrintText` "Unlocked!")
        (set `self.bIsUnlocked` true)))
    (else
      (`KismetSystemLibrary.PrintText` "Keeplooking"))))

(event `/Game/Blueprints/bp_i_interactions.NewFunction`
  (if (`self.bIsUnlocked`)
    (`/Engine/EditorBlueprintResources/StandardMacros.FlipFlop`
      (:`A`
        (bind (_direction _newtrack_0) (`Timeline|door timeline` :!label _label)
          (:`Update`
            (`SceneComponent.K2_SetRelativeRotation` (`self.SM_Bld_Door_01`) (`KismetMathLibrary.MakeRotator` 0.0 0.0 (`KismetMathLibrary.Lerp` 0.0 90.0 _newtrack_0)) false false))))
      (:`B`
        (goto _label :!via `Reverse`)))))

(fn `UserConstructionScript`)